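; AI controller for a BP_Runner pawn that fakes a player's alternating left and right power inputs.
; On possess it caches and prints the runner, and BeginPlay starts a one-shot timer with a random delay between the min and max input delays.
; SimulateInput flip-flops between SimulatePowerLeft and SimulatePowerRight on the runner, re-arming the randomized timer each time to form a continuous, irregular input loop.
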(event `self.ReceiveBeginPlay`
  (`self.SimulateInputWithDelay`))

(event `self.ReceivePossess`
  (params (PossessedPawn :type "Pawn Object Reference"))
  (bind _asbp_runner (cast `/Game/Blueprints/BP_Runner` PossessedPawn))
  (bind _output_get (set `self.OwningRunner` _asbp_runner))
  (`KismetSystemLibrary.PrintString` (`KismetSystemLibrary.GetDisplayName` _output_get)))

(event `SimulateInput`
  (bind _owningrunner (`self.OwningRunner`))
  (`/Engine/EditorBlueprintResources/StandardMacros.FlipFlop`
    (:`A`
      (`/Game/Blueprints/BP_Runner.Simulate_PowerLeft` _owningrunner)
      (`self.SimulateInputWithDelay`))
    (:`B`
      (`/Game/Blueprints/BP_Runner.Simulate_PowerRight` _owningrunner)
      (`self.SimulateInputWithDelay`))))

(fn `SimulateInputWithDelay`
  (`KismetSystemLibrary.K2_SetTimerDelegate` (`|CreateDelegate` :!event `SimulateInput`) (`KismetMathLibrary.RandomFloatInRange` (`self.MinInputDelay`) (`self.MaxInputDelay`))))

(fn `UserConstructionScript`)